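; BP_Monster is a melee enemy that wanders, chases and attacks the player, and is knocked back when hurt.
; Tick updates player distance and direction, then drives walk speed and AI MoveTo from a state enum.
; Montages and animation events toggle fist capsules, which damage each character once per swing and store launch force for retrieval.
; Damage flashes the material, and death notifies the game mode before destroying the actor.
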(fn ConstructionScript)

(event Custom|Set%20WalkSpeed%20By%20State
  (bind _charactermovement (Variables|Character|GetCharacterMovement))
  ;[1 0.9856 0] Movement change according to state ( BS )
  (switch Utilities|FlowControl|Switch|SwitchonEN_Monster (Variables|Default|GetCurState)
    (:NewEnumerator1
      (Variables|/Script/Engine.CharacterMovementComponent|SetMaxWalkSpeed _charactermovement 1e+02))
    (:NewEnumerator3
      (Variables|/Script/Engine.CharacterMovementComponent|SetMaxWalkSpeed _charactermovement 1.6e+02))))

(event Custom|SaveDistAndDir
  (bind _returnvalue (Game|GetPlayerCharacter 0))
  (bind _returnvalue_2 (Transformation|GetActorLocation))
  (bind _returnvalue_3 (Transformation|GetActorLocation _returnvalue))
  (bind _returnvalue_4 (- _returnvalue_3 _returnvalue_2))
  (bind (_x _y) (Math|Vector|BreakVector _returnvalue_4))
  (bind _returnvalue_5 (Math|Vector|MakeVector _x _y 0.0))
  ;[1 0.9744 0] Monster Move / IsDeathCharacter
  ;;[1 1 1] IsDeathCharacter
  (bind _asbp_character (Utilities|Casting|CastToBP_Character _returnvalue))
  (Variables|Default|SetIsDeathCharacter (Variables|/Game/BluePrint/Charactor/BP_Character.BP_Character_C|GetbIsDeath _asbp_character))
  ;;[1 1 1] Character destination Init
  (Variables|Default|SetPlayerLoc (Transformation|GetActorLocation (Game|GetPlayerCharacter 0)))
  (Variables|Default|SetDistancePlayerCharacter (Math|Vector|VectorLength _returnvalue_5))
  (Variables|Default|SetDirToPlayerCharacter (Math|Vector|Normalize _returnvalue_5)))

(event Custom|Chase
  ;[1 0.8874 0] Chase
  (AI|AIMoveTo self (Variables|Default|GetPlayerLoc) 0 1.3e+02 false
    (:then
      (if (>= (Variables|Default|GetDistancePlayerCharacter) 5e+02)
        _
        (else
          (Utilities|FlowControl|Sequence
            (:then_0
              (goto _label Reset))
            (:then_1
              _))))
      (Utilities|FlowControl|DoOnce false :!label _label
        (:Completed
          (Utilities|FlowControl|RetriggerableDelay 5.0)
          (Components|Movement|StopMovementImmediately (Variables|Character|GetCharacterMovement))
          (Variables|Default|SetCurState "NewEnumerator1"))))
    (:OnSuccess
      (Variables|Default|SetCurState "NewEnumerator4")
      (Animation|Montage|PlayMontage (Variables|Character|GetMesh) "/Game/Animation/AnimsMonster/AM/AM_MonsterAttack.AM_MonsterAttack"
        (:OnCompleted
          (CallFunction|NextMoveDecision))))))

(event Custom|NextMoveDecision
  ;[0.9835 1 0.01151] Chase Init
  (if (>= (Variables|Default|GetDistancePlayerCharacter) 5e+02)
    (Variables|Default|SetCurState "NewEnumerator1")
    (else
      (Variables|Default|SetCurState "NewEnumerator3"))))

(event Custom|Random%20Movement
  ;[1 0.8873 0] Map Random Movement
  (Utilities|FlowControl|DoOnce false :!label _label
    (:Completed
      (if (Utilities|Enum|Equal(Enum) (Variables|Default|GetCurState) "NewEnumerator1")
        (Variables|Default|SetisMoving? true)
        (bind _randomlocation (Class|NavigationSystemV1|GetRandomLocationinNavigableRadius (Transformation|GetActorLocation) 1.5e+03 0 0))
        (AI|AIMoveTo self _randomlocation 0 5.0 false
          (:OnSuccess
            _)
          (:OnFail
            _))
        (Variables|Default|SetisMoving? false)
        (Utilities|FlowControl|Delay (Math|Random|RandomFloatinRange 1.0 4.0))
        (goto _label Reset)))))

(event EventTick
  (params (DeltaSeconds :type Float%20%28single-precision%29))
  ;[0.9888 1 0] Monster Chase and Attack
  (CallFunction|SaveDistandDir)
  (CallFunction|SetWalkSpeedbyState)
  (switch Utilities|FlowControl|Switch|SwitchonEN_Monster (Variables|Default|GetCurState)
    (:NewEnumerator1
      (CallFunction|RandomMovement))
    (:NewEnumerator3
      (CallFunction|Chase))))

(event Custom|ChangeDamageColor
  ;[0.2397 0 1] Take Damage
  ;;[0.3685 0 1] Take Damage Color
  (Rendering|Material|SetMaterial (Variables|Character|GetMesh) 0 "/Game/Asset/Monster/warrok_MAT_Inst.warrok_MAT_Inst")
  (Utilities|FlowControl|Delay 0.2)
  (Rendering|Material|SetMaterial (Variables|Character|GetMesh) 0 "/Game/Asset/Monster/warrok_MAT.warrok_MAT"))

(event Game|Damage|EventAnyDamage
  (params (Damage :type Float%20%28single-precision%29) (DamageType :type Damage%20Type%20Object%20Reference) (InstigatedBy :type Controller%20Object%20Reference) (DamageCauser :type Actor%20Object%20Reference))
  (bind _dirtoplayercharacter (Variables|Default|GetDirToPlayerCharacter))
  (bind _returnvalue (* _dirtoplayercharacter -1.0))
  (bind _returnvalue_2 (Math|Vector|Normalize _returnvalue))
  (bind (_x _y) (Math|Vector|BreakVector _returnvalue_2))
  ;[0.2397 0 1] Take Damage
  (if (Utilities|Enum|NotEqual(Enum) (Variables|Default|GetCurState) "NewEnumerator5")
    (Variables|Default|SetCurState "NewEnumerator6")
    (Variables|Default|SetNot%20Attacking true)
    (Components|Movement|StopMovementImmediately (Variables|Character|GetCharacterMovement))
    (Character|LaunchCharacter (* (Math|Vector|MakeVector _x _y 0.0) 1e+03) false false)
    (Collision|SetCollisionEnabled (Variables|Default|GetLeft%20Capsule) "NoCollision")
    (bind _output_get (Variables|Default|SetHP (- (Variables|Default|GetHP) Damage)))
    (CallFunction|ChangeDamageColor)
    (if (<= _output_get 0.0)
      (Animation|PlayAnimMontage "/Game/Animation/AnimsMonster/AM/AM_MonsterDead.AM_MonsterDead" 1.0 "None")
      (Variables|Default|SetCurState "NewEnumerator5")
      (Collision|SetCollisionEnabled (Variables|Default|GetOverlap%20Capsule) "NoCollision")
      (Class|BPIGamemodeMP|RemoveOneEnemy(Message) (Game|GetGameMode))
      (Utilities|FlowControl|Delay 3.0)
      (Actor|DestroyActor)
      (else
        (Animation|Montage|PlayMontage (Variables|Character|GetMesh) "/Game/Animation/AnimsMonster/AM/AM_NuckBack_Montage.AM_NuckBack_Montage"
          (:OnCompleted
            _)
          (:OnInterrupted
            _))
        (Variables|Default|SetCurState "NewEnumerator3")))))

(event OnComponentBeginOverlap(RightCapsule)
  (params (OverlappedComponent :type Primitive%20Component%20Object%20Reference) (OtherActor :type Actor%20Object%20Reference) (OtherComp :type Primitive%20Component%20Object%20Reference) (OtherBodyIndex :type Integer) (bFromSweep :type Boolean) (SweepResult :type Hit%20Result%20Structure%20%28by%20ref%29))
  ;[1 0 0] No conflict myself / Apply Damage
  (if (!= OtherActor self)
    (bind _asbp_character (Utilities|Casting|CastToBP_Character OtherActor)) ; 컴퓨터에 동시성은 없다 무조건 1번 맞고 다음 맞는다
    ;;[1 0 0] Did the character take damage?
    (if (== (Utilities|Array|FindItem (Variables|Default|GetHittedActor) _asbp_character) -1)
      (Utilities|Array|AddUnique (Variables|Default|GetHittedActor) _asbp_character) ; 1번만 추가하도록 하는 함수
      (CallFunction|OnceDealingDamageDetection))))

(event OnComponentBeginOverlap(LeftCapsule)
  (params (OverlappedComponent :type Primitive%20Component%20Object%20Reference) (OtherActor :type Actor%20Object%20Reference) (OtherComp :type Primitive%20Component%20Object%20Reference) (OtherBodyIndex :type Integer) (bFromSweep :type Boolean) (SweepResult :type Hit%20Result%20Structure%20%28by%20ref%29))
  ;[1 0 0] No conflict myself / Apply Damage
  (if (!= OtherActor self)
    (bind _asbp_character (Utilities|Casting|CastToBP_Character (stale OnComponentBeginOverlap(RightCapsule) OtherActor))) ; 컴퓨터에 동시성은 없다 무조건 1번 맞고 다음 맞는다
    ;;[1 0 0] Did the character take damage?
    (if (== (Utilities|Array|FindItem (Variables|Default|GetHittedActor) _asbp_character) -1)
      (Utilities|Array|AddUnique (Variables|Default|GetHittedActor) _asbp_character) ; 1번만 추가하도록 하는 함수
      (CallFunction|OnceDealingDamageDetection))))

(event OnComponentBeginOverlap(OverlapCapsule)
  (params (OverlappedComponent :type Primitive%20Component%20Object%20Reference) (OtherActor :type Actor%20Object%20Reference) (OtherComp :type Primitive%20Component%20Object%20Reference) (OtherBodyIndex :type Integer) (bFromSweep :type Boolean) (SweepResult :type Hit%20Result%20Structure%20%28by%20ref%29))
  (bind _dirtoplayercharacter (Variables|Default|GetDirToPlayerCharacter))
  (bind (_x _y) (Math|Vector|BreakVector _dirtoplayercharacter))
  ;[1 0 0] Overlap Damage
  (Variables|Default|SetlaunchPower (* (Math|Vector|MakeVector _x _y 5e+01) "350.000000,0,1.000000"))
  (Game|Damage|ApplyDamage OtherActor 1e+01 0 self))

(event Custom|Attack_Start
  ;[1 0 0] Collision Check
  (Collision|SetCollisionEnabled (Variables|Default|GetRight%20Capsule) "QueryAndPhysics"))

(event Custom|Attack_End
  ;[1 0 0] Collision Check
  (Collision|SetCollisionEnabled (Variables|Default|GetLeft%20Capsule) "NoCollision")
  ;;[1 0 0] initialization Damage
  (Utilities|Array|Clear (Variables|Default|GetHittedActor)))

(event Custom|NextActionDecision
  ;[1 0 0] Notify Attack Togle / TODO: 기능이 중복된 로직이 있다.
  (Variables|Default|SetNot%20Attacking true) ; 스테이트 열거형으로 교체를 하는 것이 더 좋다.
  (if (Variables|Default|GetIsDeathCharacter)
    (Variables|Default|SetCurState "NewEnumerator1")
    (elif (> (Variables|Default|GetDistancePlayerCharacter) 1.3e+02)
      (Variables|Default|SetCurState "NewEnumerator3")
      (else
        (Variables|Default|SetCurState "NewEnumerator4")
        (Transformation|SetActorRotation (Math|Conversions|RotationFromXVector (Variables|Default|GetDirToPlayerCharacter)))
        (Animation|PlayAnimMontage "/Game/Animation/AnimsMonster/AM/AM_MonsterAttack.AM_MonsterAttack" 1.0 "None")
        (Variables|Default|SetNot%20Attacking false)))))

(event Custom|OnAnimEndAttack
  ;[1 0 0] Notify Attack Togle / TODO: 기능이 중복된 로직이 있다.
  ;;[1 0 0] Attack End
  (CallFunction|NextActionDecision))

(event Custom|Once%20Dealing%20Damage%20detection
  (bind _dirtoplayercharacter (Variables|Default|GetDirToPlayerCharacter))
  (bind (_x _y) (Math|Vector|BreakVector _dirtoplayercharacter))
  ;[1 0 0] Attack Damage Detection
  (for _array_element (Variables|Default|GetHittedActor)
    (Variables|Default|SetlaunchPower (* (Math|Vector|MakeVector _x _y 1e+02) "500.000000,0,1.000000"))
    (Game|Damage|ApplyDamage _array_element (Variables|Default|GetAttackDamage) 0 self)))

(event Custom|Notify_NuckBack
  ;[1 0 0] Notify Attack Togle / TODO: 기능이 중복된 로직이 있다.
  ;;[1 0 0] Knock Back End
  (CallFunction|NextActionDecision))

(fn GetLauchForece
  (return (Variables|Default|GetlaunchPower)))