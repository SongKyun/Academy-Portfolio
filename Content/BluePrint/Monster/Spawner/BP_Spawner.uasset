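; BP_Spawner is a monster spawner actor that places BP_Monster enemies at random points inside its EnnemiesSpawnZone box.
; On BeginPlay it registers itself with the game mode through a message call.
; Its SpawnOneEnemy event asks the game mode whether another enemy is allowed, spawns one with AI if so, then reports the addition back to the game mode.
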(event Custom|SpawnOneEnemy
  (bind _ennemiesspawnzone (Variables|Default|GetEnnemiesSpawnZone))
  ;[1 0 0.6634] Spawn Enemy
  (bind _bresult (Class|BPIGamemodeMP|CanSpawnOneEnemy(Message) (Game|GetGameMode)))
  (if _bresult
    (AI|SpawnAIFromClass "/Game/BluePrint/Monster/BP_Monster.BP_Monster_C" 0 (Math|Random|RandomPointinBoundingBox (Transformation|GetWorldLocation _ennemiesspawnzone) (Components|Box|GetScaledBoxExtent _ennemiesspawnzone)) "0, 0, 0" false 0)
    (Class|BPIGamemodeMP|AddOneEnemy(Message) (Game|GetGameMode))))

(event EventBeginPlay
  ;[1 0.01124 0.8091] Send reference to gamemode
  (Class|BPIGamemodeMP|ResisterSpawner(Message) (Game|GetGameMode) self))

(fn ConstructionScript)