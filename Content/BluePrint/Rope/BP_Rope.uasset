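; BP_Rope is a rope actor that builds its shape along a spline in the construction script.
; A loop adds a Z-forward spline mesh component per index, fitting it between that spline point and the next using local locations and tangents.
; The loop's upper bound is the point count plus two, so it runs past the last spline point.
; The event graph holds only disabled default events, with no runtime logic.
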(event EventBeginPlay)

(event Collision|EventActorBeginOverlap
  (params (OtherActor :type Actor%20Object%20Reference)))

(event EventTick
  (params (DeltaSeconds :type Float%20%28single-precision%29)))

(fn ConstructionScript
  (bind _spline (Variables|Default|GetSpline))
  (for _index (range 0 (+ (Spline|GetNumberOfSplinePoints (Variables|Default|GetSpline)) 2)) ; startindex부터 stopindex까지 각 인덱스에 대해 loopbody를 실행합니다.\ninclusive 포함한
    (bind _returnvalue (AddComponent|AddSplineMeshComponent false)) ; 새 구성 요소를 만들고 액터에 소유권을 할당합니다. \n이것은 자동 연결을 위해 호출되어 생성된 첫 번째 구성 요소가 루트가 되도록 합니다.\n bManualAttachment가 설정되면 자동 연결을 건너뛰고 결과 구성 요소를 직접 연결하는 것은 사용자에게 달려 있습니다.
    (SplineMesh|SetForwardAxis _returnvalue "Z" true) ; Axis 중심선
    (SplineMesh|SetStartandEnd _returnvalue (.Location (Spline|GetLocationandTangentatSplinePoint _spline _index "Local")) (.Tangent (Spline|GetLocationandTangentatSplinePoint _spline _index "Local")) (.Location (Spline|GetLocationandTangentatSplinePoint _spline (+ _index 1) "Local")) (.Tangent (Spline|GetLocationandTangentatSplinePoint _spline (+ _index 1) "Local")) true :!class /Script/Engine.SplineMeshComponent)))